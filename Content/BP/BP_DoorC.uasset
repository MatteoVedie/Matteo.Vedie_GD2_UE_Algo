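; BP_DoorC is a door Blueprint that swings open or closed and switches a referenced light along with it.
; Activate checks the Open flag, turning the light off and opening the door when closed, or turning it on and closing it when open.
; OpenDoor and CloseDoor update the flag and each play a separate timeline from the start, driving the Door component's relative yaw.
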(event Custom|OpenDoor
  (Variables|Default|SetOpen? true)
  (bind _opendoor (Timeline|OUI PlayFromStart)
    (:Update
      (Transformation|SetRelativeRotation (Variables|Default|GetDoor) (Math|Rotator|MakeRotator 0.0 0.0 _opendoor) false false))))

(event Custom|CloseDoor
  (Variables|Default|SetOpen? false)
  (bind _newtrack_0 (Timeline|NON PlayFromStart)
    (:Update
      (Transformation|SetRelativeRotation (Variables|Default|GetDoor) (Math|Rotator|MakeRotator 0.0 0.0 _newtrack_0) false false))))

(event EventActivate
  (bind _lightref (Variables|Default|GetLightREF))
  (if (Variables|Default|GetOpen?)
    (Default|Lighton _lightref)
    (CallFunction|CloseDoor)
    (else
      (Default|LightOff _lightref)
      (CallFunction|OpenDoor))))

(fn ConstructionScript)