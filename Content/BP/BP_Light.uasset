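; Light actor Blueprint whose Light component is switched on and off through a counter named DoorNumber.
; Light Off increments the counter and hides the light while the count is above zero.
; Light On decrements it and shows the light only when the count returns to zero, so overlapping off requests must all be released first.
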(fn ConstructionScript)

(fn LightOff
  (bind _result (Math|Integer|IncrementInt (Variables|Default|GetDoorNumber))
    (:%20%20
      (if (> _result 0)
        (Rendering|SetVisibility (Variables|Default|GetLight) false false)))))

(fn Lighton
  (bind _result (Math|Integer|DecrementInt (Variables|Default|GetDoorNumber))
    (:%20%20
      (if (== _result 0)
        (Rendering|SetVisibility (Variables|Default|GetLight) true false)))))